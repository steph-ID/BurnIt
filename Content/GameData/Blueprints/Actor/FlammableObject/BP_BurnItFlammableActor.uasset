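; Burnable world actor for BurnIt that catches fire, spreads heat to neighbors and leaves an ash pile.
; Ignite and Extinguish toggle a Niagara flame on the mesh, while a dynamic overlay material shows heat.
; Propagate overlaps a sphere and adds curve-scaled heat to nearby flammable actors, flagging close flame contact and drawing debug lines.
; DropAsh swaps the actor for valued ash, and the FlammableComponent sends points when the game state reaches Ending.
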(event OnComponentBeginOverlap(StaticMesh)
  (params (OverlappedComponent :type Primitive%20Component%20Object%20Reference) (OtherActor :type Actor%20Object%20Reference) (OtherComp :type Primitive%20Component%20Object%20Reference) (OtherBodyIndex :type Integer) (bFromSweep :type Boolean) (SweepResult :type Hit%20Result%20Structure%20%28by%20ref%29)))

(event EventBeginPlay
  (bind _returnvalue (Rendering|Material|CreateDynamicMaterialInstance "/Game/GameData/Materials/MI_HeatedOverlay.MI_HeatedOverlay" "None" "None" :!class /Script/Engine.KismetMaterialLibrary))
  (bind _output_get (Variables|Default|SetOverlayMaterial _returnvalue))
  (Rendering|Material|SetScalarParameterValue _output_get "Visibility" (Class|BurnItFlammableComponent|GetHeatedMaterialVisibility (Class|BurnItFlammableActor|GetFlammableComponent)) :!class /Script/Engine.MaterialInstanceDynamic)
  (Rendering|Material|SetOverlayMaterial (Variables|Default|GetStaticMesh) _returnvalue :!class /Script/Engine.MeshComponent)
  (bind _asburn_it_game_state_base (Utilities|Casting|CastToBurnItGameStateBase (Game|GetGameState)))
  (EventDispatchers|BindEventtoOnGameStateChange _asburn_it_game_state_base (delegate EventGameStateChanged))
  (Components|Activation|SetActive (Variables|Default|GetSphere) false false))

(event EventPropagate
  (bind _sphere (Variables|Default|GetSphere))
  (bind _flammablecomponent (Variables|Default|GetFlammableComponent))
  (bind _staticmesh (Variables|Default|GetStaticMesh))
  (bind _returnvalue (Class|BurnItFlammableComponent|GetBurnTemperature _flammablecomponent))
  (bind _returnvalue_2 (Transformation|GetWorldLocation _staticmesh))
  (Components|Activation|SetActive _sphere true false)
  (bind _outcomponents (Class|KismetSystemLibrary|ComponentOverlapComponents _sphere (Math|Transform|MakeTransform (Transformation|GetWorldLocation _sphere) "0, 0, 0" "1.000000,1.000000,1.000000") (Variables|Default|GetObject%20Types) "/Script/Engine.StaticMeshComponent"))
  (for _array_element _outcomponents
    (bind _asburn_it_flammable_actor (Utilities|Casting|CastToBurnItFlammableActor (Components|GetOwner _array_element)))
    (Rendering|Debug|DrawDebugLine (+ _returnvalue_2 (* (.BoxExtent (Collision|GetComponentBounds _staticmesh)) (Math|Vector|GetUnitDirection(Vector) _returnvalue_2 (Transformation|GetWorldLocation _array_element)))) (.OutPointOnBody (Collision|GetClosestPointonCollision _array_element (+ _returnvalue_2 (* (.BoxExtent (Collision|GetComponentBounds _staticmesh)) (Math|Vector|GetUnitDirection(Vector) _returnvalue_2 (Transformation|GetWorldLocation _array_element)))) "None")) "(R=0.240757,G=0.000000,B=1.000000,A=1.000000)" 5.0 1.0)
    (if (<= (.ReturnValue (Collision|GetClosestPointonCollision _array_element (+ _returnvalue_2 (* (.BoxExtent (Collision|GetComponentBounds _staticmesh)) (Math|Vector|GetUnitDirection(Vector) _returnvalue_2 (Transformation|GetWorldLocation _array_element)))) "None")) 5e+01)
      (Variables|Default|SetOutgoingTemp (* _returnvalue 2.0))
      (else
        (Variables|Default|SetOutgoingTemp (* _returnvalue (Math|Curves|GetFloatValue (Variables|/Script/BurnIt.BurnItFlammableComponent|GetBurnTempFalloffCurve _flammablecomponent) (Math|Float|Clamp(Float) (Math|Float|NormalizetoRange (Transformation|GetDistanceTo _asburn_it_flammable_actor) 0.0 (Variables|Default|GetIgnitionSphereRadius))))))))
    (Class|BurnItFlammableComponent|AdjustTemperature (Variables|/Script/BurnIt.BurnItFlammableActor|GetFlammableComponent _asburn_it_flammable_actor) (* _returnvalue (Math|Curves|GetFloatValue (Variables|/Script/BurnIt.BurnItFlammableComponent|GetBurnTempFalloffCurve _flammablecomponent) (Math|Float|Clamp(Float) (Math|Float|NormalizetoRange (Transformation|GetDistanceTo _asburn_it_flammable_actor) 0.0 (Variables|Default|GetIgnitionSphereRadius))))) (<= (.ReturnValue (Collision|GetClosestPointonCollision _array_element (+ _returnvalue_2 (* (.BoxExtent (Collision|GetComponentBounds _staticmesh)) (Math|Vector|GetUnitDirection(Vector) _returnvalue_2 (Transformation|GetWorldLocation _array_element)))) "None")) 5e+01) self)))

(event EventGameStateChanged
  (params (NewGameState :type EGameState%20Enum :default "None"))
  (switch Utilities|FlowControl|Switch|SwitchonEGameState NewGameState
    (:Ending
      (Class|BurnItFlammableComponent|SendPoints (Variables|Default|GetFlammableComponent)))))

(event EventIgnite
  (bind _flamesystem (Variables|Default|GetFlameSystem))
  (Class|NiagaraFunctionLibrary|OverrideSystemUserVariableStaticMeshComponent _flamesystem "" (Variables|Default|GetStaticMesh))
  (Niagara|SetNiagaraVariable(Float) _flamesystem "Spawn.PerSecond" (Variables|Default|GetParticleSpawnRate))
  (Components|Activation|SetActive _flamesystem true false))

(event EventDropAsh
  (bind _returnvalue (Game|SpawnActorfromClass (Variables|Default|GetAshPileClass) (Math|Transform|MakeTransform (Transformation|GetWorldLocation (Variables|Default|GetStaticMesh)) (Math|Rotator|MakeRotator 0.0 0.0 (.yaw (Math|Random|RandomRotator false))) "1.000000,1.000000,1.000000") "Undefined" "MultiplyWithRoot" 0 0))
  (bind _asbp_ash_pile (Utilities|Casting|CastToBP_AshPile _returnvalue))
  (Default|SetAshValue _asbp_ash_pile (Variables|Default|GetAshValue))
  (Actor|DestroyActor))

(event EventExtinguish
  (bind _flamesystem (Variables|Default|GetFlameSystem))
  (bind _ignitionsphere (Variables|Default|GetIgnitionSphere))
  (if (Components|Activation|IsActive _flamesystem)
    (Components|Activation|SetActive _flamesystem false false)
    (Utilities|IsValid _ignitionsphere
      (:Is%20Valid
        (Components|DestroyComponent _ignitionsphere)))))

(event EventSetHeatedMaterialVisibility
  (params (NewHeatedMaterialVisibility :type Float%20%28single-precision%29))
  (bind _overlaymaterial (Variables|Default|GetOverlayMaterial))
  (Rendering|Material|SetScalarParameterValue _overlaymaterial "Visibility" NewHeatedMaterialVisibility :!class /Script/Engine.MaterialInstanceDynamic)
  (Rendering|Material|SetOverlayMaterial (Variables|Default|GetStaticMesh) _overlaymaterial :!class /Script/Engine.MeshComponent))

(event Input|KeyboardEvents|DebugKeyT
  (params (Key :type Key%20Structure :default "None") (ActionValue :type Input%20Action%20Value%20Structure))
  (bind _flamesystem (Variables|Default|GetFlameSystem))
  (:Pressed
    (Niagara|SetNiagaraVariable(Float) _flamesystem "Spawn.PerSecond" (Variables|Default|GetParticleSpawnRate))
    (Components|Activation|SetActive _flamesystem true false)))

(fn ConstructionScript)