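; Exit portal actor that appears when the round reaches its ending state and shows a leave message to the player touching it.
; On BeginPlay it binds to the game state's change event, hiding itself without collision while Waiting and showing with collision during Ending.
; Capsule overlap by a BurnIt character reaches that player's HUD overlay widget and sends it the round-leave row from the UI messages DataTable.
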(event `self.ReceiveBeginPlay`
  (bind _asburn_it_game_state_base (cast `BurnItGameStateBase` (`GameplayStatics.GetGameState`)))
  (add `BurnItGameStateBase.OnGameStateChange` _asburn_it_game_state_base (delegate `OnGameStateChange_Event`)))

(event `OnGameStateChange_Event`
  (params (NewGameState :type "EGameState Enum" :default "None"))
  (switch `EGameState` NewGameState
    (:`Waiting`
      (`self.SetActorHiddenInGame` true)
      (`self.SetActorEnableCollision` false))
    (:`Ending`
      (`self.SetActorHiddenInGame` false)
      (`self.SetActorEnableCollision` true))))

(event `self.Capsule.OnComponentBeginOverlap`
  (params (OverlappedComponent :type "PrimitiveComponent Object Reference") (OtherActor :type "Actor Object Reference") (OtherComp :type "PrimitiveComponent Object Reference") (OtherBodyIndex :type Integer) (bFromSweep :type Boolean) (SweepResult :type "HitResult Structure (by ref)"))
  (bind _asburn_it_character (cast `BurnItCharacter` OtherActor))
  (bind _asbp_burn_it_player_controller (cast `/Game/GameData/Blueprints/Core/BP_BurnItPlayerController` (`Pawn.GetController` _asburn_it_character)))
  (bind _asbp_burn_it_hud (cast `/Game/GameData/UI/HUD/BP_BurnItHUD` (`PlayerController.GetHUD` _asbp_burn_it_player_controller)))
  (message `/Game/GameData/Blueprints/Interface/BPI_UI_Message.ReceiveMessage` (`BurnItHUD.GetOverlayWidget` _asbp_burn_it_hud) "/Game/GameData/Data/UI/DT_UI_Messages.DT_UI_Messages" "Round_Leave"))

(fn `UserConstructionScript`)