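; Flammable actor that shows heat, burns with a Niagara flame and turns into an ash pile, driven by Ignite, Extinguish and DropAsh events.
; A dynamic overlay material on the mesh displays heat through its Visibility parameter, initialized from the flammable component.
; Ignite or debug key T starts the flame at ParticleSpawnRate, and Extinguish deactivates it.
; DropAsh spawns a randomly yawed ash pile, passes it AshValue and destroys the actor.
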(event OnComponentBeginOverlap(StaticMesh)
  (params (OverlappedComponent :type Primitive%20Component%20Object%20Reference) (OtherActor :type Actor%20Object%20Reference) (OtherComp :type Primitive%20Component%20Object%20Reference) (OtherBodyIndex :type Integer) (bFromSweep :type Boolean) (SweepResult :type Hit%20Result%20Structure%20%28by%20ref%29)))

(event EventBeginPlay
  (bind _returnvalue (Rendering|Material|CreateDynamicMaterialInstance "/Game/GameData/Materials/MI_HeatedOverlay.MI_HeatedOverlay" "None" "None" :!class /Script/Engine.KismetMaterialLibrary))
  (bind _output_get (Variables|Default|SetOverlayMaterial _returnvalue))
  (Rendering|Material|SetScalarParameterValue _output_get "Visibility" (Class|BurnItFlammableComponent|GetHeatedMaterialVisibility (Class|BurnItFlammableActor|GetFlammableComponent)) :!class /Script/Engine.MaterialInstanceDynamic)
  (Rendering|Material|SetOverlayMaterial (Variables|Default|GetStaticMesh) _returnvalue :!class /Script/Engine.MeshComponent))

(event EventIgnite
  (bind _flamesystem (Variables|Default|GetFlameSystem))
  (Niagara|SetNiagaraVariable(Float) _flamesystem "Spawn.PerSecond" (Variables|Default|GetParticleSpawnRate))
  (Components|Activation|SetActive _flamesystem true false))

(event EventDropAsh
  (bind _returnvalue (Game|SpawnActorfromClass (Variables|Default|GetAshPileClass) (Math|Transform|MakeTransform (Transformation|GetWorldLocation (Variables|Default|GetStaticMesh)) (Math|Rotator|MakeRotator 0.0 0.0 (.yaw (Math|Random|RandomRotator false))) "1.000000,1.000000,1.000000") "Undefined" "MultiplyWithRoot" 0 0))
  (bind _asbp_ash_pile (Utilities|Casting|CastToBP_AshPile _returnvalue))
  (Default|SetAshValue _asbp_ash_pile (Variables|Default|GetAshValue))
  (Actor|DestroyActor))

(event EventExtinguish
  (bind _flamesystem (Variables|Default|GetFlameSystem))
  (if (Components|Activation|IsActive _flamesystem)
    (Components|Activation|SetActive _flamesystem false false)))

(event EventSetHeatedMaterialVisibility
  (params (NewHeatedMaterialVisibility :type Float%20%28single-precision%29))
  (bind _overlaymaterial (Variables|Default|GetOverlayMaterial))
  (Rendering|Material|SetScalarParameterValue _overlaymaterial "Visibility" NewHeatedMaterialVisibility :!class /Script/Engine.MaterialInstanceDynamic)
  (Rendering|Material|SetOverlayMaterial (Variables|Default|GetStaticMesh) _overlaymaterial :!class /Script/Engine.MeshComponent))

(event Input|KeyboardEvents|DebugKeyT
  (params (Key :type Key%20Structure) (ActionValue :type Input%20Action%20Value%20Structure))
  (bind _flamesystem (Variables|Default|GetFlameSystem))
  (:Pressed
    (Niagara|SetNiagaraVariable(Float) _flamesystem "Spawn.PerSecond" (Variables|Default|GetParticleSpawnRate))
    (Components|Activation|SetActive _flamesystem true false)))

(fn ConstructionScript)

(fn CalculateParticleSpawnRate)