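; Ignition device Blueprint that projects flame heat onto flammable actors.
; When the device-triggered event fires with non-negative fuel, it sphere-traces from the Niagara flame effect along its forward vector out to FlameRange.
; Each BP_BurnItFlammableActor hit has its temperature raised, scaled by hit distance through the DeviceHeatRamp curve, and is flagged as touched by flames.
; Tick is empty, and several disconnected experiments, including a particle-speed trace loop, never run.
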(event `self.ReceiveBeginPlay`
  (add `self.OnDeviceTriggered` (delegate `OnDeviceTriggered_Event`)))

(event `self.ReceiveTick`
  (params (DeltaSeconds :type "Float (single-precision)")))

(event `OnDeviceTriggered_Event`
  (bind _flamefxniagaracomponent (`self.FlameFxNiagaraComponent`))
  (bind _returnvalue (`SceneComponent.K2_GetComponentLocation` _flamefxniagaracomponent))
  (bind _output_get (set `self.HasFuel` (>= (`self.GetFuel`) 0.0)))
  (if _output_get
    (set `self.CurrentLocation` _returnvalue)
    (bind (_outhits _returnvalue_2) (`KismetSystemLibrary.SphereTraceMulti` _returnvalue (+ _returnvalue (* (`KismetMathLibrary.GetForwardVector` (`SceneComponent.K2_GetComponentRotation` _flamefxniagaracomponent)) (`self.FlameRange`))) 8.0 "TraceTypeQuery3"))
    (if _returnvalue_2
      (for _array_element _outhits
        (bind (_bblockinghit _binitialoverlap _time _distance _location _impactpoint _normal _impactnormal _physmat _hitactor) (`GameplayStatics.BreakHitResult` _array_element))
        (bind _asbp_burn_it_flammable_actor (cast `/Game/GameData/Blueprints/Actor/FlammableObject/BP_BurnItFlammableActor` _hitactor))
        (`BurnItFlammableComponent.AdjustTemperature` (`BurnItFlammableActor.GetFlammableComponent` _asbp_burn_it_flammable_actor) (* (`self.Temperature`) (`CurveFloat.GetFloatValue` (`self.DeviceHeatRamp`) (`KismetMathLibrary.NormalizeToRange` (`KismetMathLibrary.Vector_Distance` _location (`self.CurrentLocation`)) 0.0 (`self.FlameRange`)))) true null)))))

(fn `UserConstructionScript`)