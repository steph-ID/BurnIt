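; BP_IgnitionInterface is an ignition interface for raising temperature, exposing an empty RaiseTemperature function.
; Its graphs also hold disconnected flame-device logic that never runs.
; That logic would heat hit BP_BurnItFlammableActor instances through their flammable component's AdjustTemperature, scaling Temperature by a DeviceHeatRamp curve over distance from the flame Niagara component within FlameRange.
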(fn `RaiseTemperature`)