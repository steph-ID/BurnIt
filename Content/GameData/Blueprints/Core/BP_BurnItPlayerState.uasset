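; BP_BurnItPlayerState is a player state Blueprint that handles name changes and exposes player and round data.
; Setting a name calls the game mode's ChangeName with the player's controller, then calls SetDisplayName.
; An event applies player data from a load through SetPlayerData, while two wrapper functions return the player and round data structs.
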(event `self.ReceiveBeginPlay`)

(event `/Game/GameData/Blueprints/Interface/BPI_Player.SetPlayerName`
  (params (NewPlayerName :type String))
  (`GameModeBase.ChangeName` (`GameplayStatics.GetGameMode`) (`self.GetPlayerController`) NewPlayerName false)
  (`self.SetDisplayName`))

(event `/Game/GameData/Blueprints/Interface/BPI_Player.SetPlayerDataFromLoad`
  (params (PlayerData :type "PlayerData Structure"))
  (`self.SetPlayerData` PlayerData))

(fn `GetPlayerDataStruct`
  (returns (PlayerData :type "PlayerData Structure"))
  (bind _returnvalue (`self.GetPlayerData`))
  (return _returnvalue))

(fn `GetRoundDataStruct`
  (returns (RoundHistory :type "RoundData Structure"))
  (bind _returnvalue (`self.GetRoundData`))
  (return _returnvalue))

(fn `UserConstructionScript`)