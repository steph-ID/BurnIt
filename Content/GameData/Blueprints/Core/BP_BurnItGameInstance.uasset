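; Game instance that owns save and load for the game, exposing the current save data and player save.
; On Init it loads or creates the save-slot index object.
; Game data loads or saves by slot name, sync or async, with only async loads firing OnGameLoaded.
; A missing save gets a new object and registers its slot in memory; the index is never written here, and CreateNewSave is empty.
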(event `/Game/GameData/Data/SaveGame/BPI_SaveGame.LoadGameSaveSlots`
  ;[0.05127 0.05127 0.05127] Load all available save slots
  (bind _returnvalue (`GameplayStatics.DoesSaveGameExist` (`self.AvailableSaveGameSlotName`)))
  (if _returnvalue
    (bind _returnvalue_2 (`GameplayStatics.LoadGameFromSlot` (`self.AvailableSaveGameSlotName`)))
    (bind _asbp_save_game_slots (cast `/Game/GameData/Data/SaveGame/BP_SaveGameSlots` _returnvalue_2))
    (set `self.AvailableSaveSlots` _asbp_save_game_slots)
    (else
      (bind _returnvalue_3 (`GameplayStatics.CreateSaveGameObject` "/Game/GameData/Data/SaveGame/BP_SaveGameSlots.BP_SaveGameSlots_C"))
      (set `self.AvailableSaveSlots` _returnvalue_3))))

(event `self.ReceiveInit`
  ;[0.05127 0.05127 0.05127] Initial load
  (`/Game/GameData/Data/SaveGame/BPI_SaveGame.LoadGameSaveSlots`))

(event `/Game/GameData/Data/SaveGame/BPI_SaveGame.LoadGameData`
  (params (Async :type Boolean))
  ;[0.05127 0.05127 0.05127] Load game
  (bind _returnvalue (`GameplayStatics.DoesSaveGameExist` (`self.Slot Name`)))
  (if _returnvalue
    (if Async
      (bind _savegame (`AsyncActionHandleSaveGame.AsyncLoadGameFromSlot` (`self.Slot Name`))
        (:`Completed`
          (bind _asbp_save_game (cast `/Game/GameData/Data/SaveGame/BP_SaveGame` _savegame))
          (set `self.SavedData` _asbp_save_game)
          (`self.OnGameLoaded`)))
      (else
        (bind _returnvalue_2 (`GameplayStatics.LoadGameFromSlot` (`self.Slot Name`)))
        (bind _asbp_save_game_2 (cast `/Game/GameData/Data/SaveGame/BP_SaveGame` _returnvalue_2))
        (set `self.SavedData` _asbp_save_game_2)))
    (else
      (bind _returnvalue_3 (`GameplayStatics.CreateSaveGameObject` "/Game/GameData/Data/SaveGame/BP_SaveGame.BP_SaveGame_C"))
      (set `self.SavedData` _returnvalue_3)
      (`KismetArrayLibrary.Array_AddUnique` (`/Game/GameData/Data/SaveGame/BP_SaveGameSlots.SavedGameSlots` (`self.AvailableSaveSlots`)) (`self.Slot Name`)))))

(event `/Game/GameData/Data/SaveGame/BPI_SaveGame.SaveGameData`
  (params (Async :type Boolean))
  ;[0.05127 0.05127 0.05127] Save game
  (if Async
    (`AsyncActionHandleSaveGame.AsyncSaveGameToSlot` (`self.SavedData`) (`self.Slot Name`))
    (else
      (`GameplayStatics.SaveGameToSlot` (`self.SavedData`) (`self.Slot Name`)))))

(event `/Game/GameData/Data/SaveGame/BPI_SaveGame.SavePlayer`
  (params (PlayerData :type "/Game/GameData/Data/SaveGame/S_PlayerSave Structure") (Async :type Boolean))
  (set `/Game/GameData/Data/SaveGame/BP_SaveGame.PlayerSave` PlayerData (`self.SavedData`))
  (`self.SaveGameData` Async))

(event `/Game/GameData/Data/SaveGame/BPI_SaveGame.CreateNewSave`
  (params (CharacterName :type Text)))

(fn `GetGameData`
  (returns (SaveGameData :type "BurnItSaveGame Object Reference"))
  (return (`self.SavedData`)))

(fn `GetPlayerSave`
  (returns (PlayerData :type "/Game/GameData/Data/SaveGame/S_PlayerSave Structure"))
  (return (`/Game/GameData/Data/SaveGame/BP_SaveGame.PlayerSave` (`self.SavedData`))))