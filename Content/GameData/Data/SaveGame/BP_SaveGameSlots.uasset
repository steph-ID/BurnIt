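; Save game slot registry that holds a map of saved games and provides them as an array ordered by last-saved date.
; SortSaveSlotArray copies the map values into SavedGameSlotsArray, then repeats bubble-sort swap passes until none occur, returning newest first.
; SortSaveFiles is an unfinished pivot-partition sort using CompareDates; its alternative loop with CompareDateWithPivot and the EventGraph array-filling logic never run.
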(fn `CompareDates`
  (params (First :type "/Game/GameData/Data/SaveGame/S_SavedGame Structure (by ref)") (Pivot :type "/Game/GameData/Data/SaveGame/S_SavedGame Structure"))
  (returns (ReturnValue :type Boolean))
  (return (> (`.LastSaved_28_BDD0813A451AF060352070A71CB2B6BF` (break `/Game/GameData/Data/SaveGame/S_SavedGame` First)) (`.LastSaved_28_BDD0813A451AF060352070A71CB2B6BF` (break `/Game/GameData/Data/SaveGame/S_SavedGame` Pivot)))))

(fn `CompareDateWithPivot`
  (params (S_SavedGame :type "/Game/GameData/Data/SaveGame/S_SavedGame Structure (by ref)") (TargetArray :type "Array of /Game/GameData/Data/SaveGame/S_SavedGame Structure (by ref)"))
  (returns (ReturnValue :type Boolean))
  (return (> (`.LastSaved_28_BDD0813A451AF060352070A71CB2B6BF` (break `/Game/GameData/Data/SaveGame/S_SavedGame` S_SavedGame)) (`.LastSaved_28_BDD0813A451AF060352070A71CB2B6BF` (break `/Game/GameData/Data/SaveGame/S_SavedGame` (`|GetArrayItem` (`self.SavedGameSlotsArray`) (- (`KismetArrayLibrary.Array_Length` TargetArray) 1)))))))

(fn `SortSaveFiles`
  (params (TargetArray :type "Array of /Game/GameData/Data/SaveGame/S_SavedGame Structure (by ref)"))
  (returns (ReturnValue :type Boolean))
  (locals (Pivot :type "/Game/GameData/Data/SaveGame/S_SavedGame Structure") (Above :type "Array of /Game/GameData/Data/SaveGame/S_SavedGame Structure") (Below :type "Array of /Game/GameData/Data/SaveGame/S_SavedGame Structure"))
  (bind _output_get (set `local.Pivot` (`|GetArrayItem` TargetArray (- (`KismetArrayLibrary.Array_Length` TargetArray) 1))))
  (for (_array_element _array_index) TargetArray
    (bind _returnvalue (`self.CompareDates` _array_element _output_get))
    (if _returnvalue
      (`KismetArrayLibrary.Array_Swap` (`local.Above`) _array_index)
      (else
        (`KismetArrayLibrary.Array_Swap` (`local.Below`)))))
  (if (`KismetArrayLibrary.Array_IsNotEmpty` (`local.Above`))
    _))

(fn `SortSaveSlotArray`
  (returns (SortedSaveGameSlots :type "Array of /Game/GameData/Data/SaveGame/S_SavedGame Structure"))
  (locals (SwapCount :type Integer) (i :type Integer))
  (bind _values (`BlueprintMapLibrary.Map_Values` (`self.SavedGameSlots`)))
  (bind _output_get (set `self.SavedGameSlotsArray` _values))
  (set `local.SwapCount` 0 :!label _label)
  (set `local.i` 0)
  (for (_array_element _array_index) _output_get
    (bind _returnvalue (`KismetArrayLibrary.Array_Length` _output_get))
    (if (< (`local.i`) _returnvalue)
      (bind _returnvalue_2 (`KismetMathLibrary.Clamp` (- _array_index 1) 0 _returnvalue))
      (if (> (`.LastSaved_28_BDD0813A451AF060352070A71CB2B6BF` (break `/Game/GameData/Data/SaveGame/S_SavedGame` _array_element)) (`.LastSaved_28_BDD0813A451AF060352070A71CB2B6BF` (break `/Game/GameData/Data/SaveGame/S_SavedGame` (`|GetArrayItem` _output_get _returnvalue_2))))
        (`KismetArrayLibrary.Array_Swap` _output_get _array_index _returnvalue_2)
        (`/Engine/EditorBlueprintResources/StandardMacros.IncrementInt` (`local.SwapCount`)
          (:`  `
            _)))
      (`/Engine/EditorBlueprintResources/StandardMacros.IncrementInt` (`local.i`))))
  (if (> (`local.SwapCount`) 0)
    (goto _label)
    (else
      (return (`self.SavedGameSlotsArray`)))))